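; BP_IaVehicule is an actor, named as an AI vehicle, whose only graph logic keeps it inside a box around the world origin.
; Every Tick, a Sequence checks each axis of its location against fixed, symmetric limits.
; Crossing any limit teleports it to the world origin without sweep.
; BeginPlay and the construction script are empty, and no driving or AI logic appears in these graphs.
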(event EventBeginPlay)

(event Collision|EventActorBeginOverlap
  (params (OtherActor :type Actor%20Object%20Reference)))

(event EventTick
  (params (DeltaSeconds :type Float%20%28single-precision%29))
  (Utilities|FlowControl|Sequence
    (:then_0
      (if (< (.x (Transformation|GetActorLocation)) -3e+02)
        (Transformation|SetActorLocation "0.000000, 0, 0" false true)))
    (:then_1
      (if (< (.y (Transformation|GetActorLocation)) -3e+02)
        (Transformation|SetActorLocation "0.000000,0.000000, 0" false true)))
    (:then_2
      (if (> (.x (Transformation|GetActorLocation)) 3e+02)
        (Transformation|SetActorLocation "0.000000, 0, 0" false true)))
    (:then_3
      (if (> (.y (Transformation|GetActorLocation)) 3e+02)
        (Transformation|SetActorLocation "0.000000,0.000000, 0" false true)))
    (:then_4
      (if (< (.z (Transformation|GetActorLocation)) -3e+02)
        (Transformation|SetActorLocation "0, 0, 0" false true)))
    (:then_5
      (if (> (.z (Transformation|GetActorLocation)) 3e+02)
        (Transformation|SetActorLocation "0, 0, 0" false true)))))

(fn ConstructionScript)